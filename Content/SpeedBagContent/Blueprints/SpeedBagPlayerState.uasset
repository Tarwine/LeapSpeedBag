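; SpeedBagPlayerState holds the timer and game-over state for a speed bag game.
; While the bag is active and the game is not over, Tick subtracts delta time from GameTime.
; When the countdown reaches zero, it clamps GameTime and sets IsGameOver, with no other logic in the graph.
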(event EventBeginPlay)

(event EventTick
  (params (DeltaSeconds :type Float%20%28single-precision%29))
  (if (Variables|Default|GetSpeedBagActive)
    (if (not (Variables|Default|GetIsGameOver))
      (bind _output_get (Variables|Default|SetGameTime (- (Variables|Default|GetGameTime) DeltaSeconds)))
      (if (<= _output_get 0.0)
        (Variables|Default|SetGameTime 0.0)
        (Variables|Default|SetIsGameOver true)))))

(fn ConstructionScript)