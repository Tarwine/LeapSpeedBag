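; SlipBag_BP is a slip bag station that activates when the player pawn enters its sphere trigger.
; Entering shows the bag meshes, turns off the marker particles and sets the speed bag active in the player state.
; Tick then eases the pawn to the trigger's center with VInterpTo.
; Leaving hides the meshes, restores the particles, releases the pawn and resets its punch count, game timer and active flag.
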(event OnComponentBeginOverlap(SphereTrigger)
  (params (OtherActor :type Actor%20Object%20Reference) (OtherComp :type Primitive%20Component%20Object%20Reference) (OtherBodyIndex :type Integer) (bFromSweep :type Boolean) (SweepResult :type Hit%20Result%20Structure%20%28by%20ref%29))
  ;[0.5283 1 0.5441] Enable the station when the player walks neaar
  (if (Actor|ActorHasTag OtherActor "Player")
    (bind _asspeed_bag_pawn_bp (Utilities|Casting|CastToSpeedBagPawn_BP OtherActor))
    (Variables|/Game/SpeedBagContent/Blueprints/SpeedBagPawn_BP.SpeedBagPawn_BP_C|SetAtBagStation _asspeed_bag_pawn_bp true)
    (Components|Activation|Deactivate (Variables|Default|Getprt_trigger))
    (Variables|SpeedBag|SetLerpPlayer true)
    (Variables|SpeedBag|SetPawnAtStation _asspeed_bag_pawn_bp)
    (Rendering|SetVisibility (Variables|Default|GetBase) true false)
    (Variables|/Game/SpeedBagContent/Blueprints/SpeedBagPlayerState.SpeedBagPlayerState_C|SetSpeedBagActive (Variables|/Game/SpeedBagContent/Blueprints/SpeedBagPawn_BP.SpeedBagPawn_BP_C|GetSBPlayerState _asspeed_bag_pawn_bp) true)
    (Variables|/Game/SpeedBagContent/Blueprints/SpeedBagPlayerState.SpeedBagPlayerState_C|SetIsGameOver (Variables|/Game/SpeedBagContent/Blueprints/SpeedBagPawn_BP.SpeedBagPawn_BP_C|GetSBPlayerState _asspeed_bag_pawn_bp) false)))

(event OnComponentEndOverlap(SphereTrigger)
  (params (OtherActor :type Actor%20Object%20Reference) (OtherComp :type Primitive%20Component%20Object%20Reference) (OtherBodyIndex :type Integer))
  ;[1 0.6068 0.6547] Disable the station when the player walks away
  (Utilities|IsValid (Variables|SpeedBag|GetPawnAtStation)
    (:Is%20Valid
      (Variables|/Game/SpeedBagContent/Blueprints/SpeedBagPlayerState.SpeedBagPlayerState_C|SetPunchCount (Variables|/Game/SpeedBagContent/Blueprints/SpeedBagPawn_BP.SpeedBagPawn_BP_C|GetSBPlayerState (Variables|SpeedBag|GetPawnAtStation)) 0)
      (Variables|/Game/SpeedBagContent/Blueprints/SpeedBagPlayerState.SpeedBagPlayerState_C|SetGameTime (Variables|/Game/SpeedBagContent/Blueprints/SpeedBagPawn_BP.SpeedBagPawn_BP_C|GetSBPlayerState (Variables|SpeedBag|GetPawnAtStation)) 6e+01)
      (Components|Activation|Activate (Variables|Default|Getprt_trigger) true)
      (Variables|/Game/SpeedBagContent/Blueprints/SpeedBagPlayerState.SpeedBagPlayerState_C|SetSpeedBagActive (Variables|/Game/SpeedBagContent/Blueprints/SpeedBagPawn_BP.SpeedBagPawn_BP_C|GetSBPlayerState (Variables|SpeedBag|GetPawnAtStation)) false)
      (Rendering|SetVisibility (Variables|Default|GetBase) false false)
      (Variables|SpeedBag|SetPawnAtStation 0)
      (Variables|SpeedBag|SetLerpPlayer false))))

(event EventBeginPlay)

(event Collision|EventActorBeginOverlap
  (params (OtherActor :type Actor%20Object%20Reference)))

(event EventTick
  (params (DeltaSeconds :type Float%20%28single-precision%29))
  (bind _pawnatstation (Variables|SpeedBag|GetPawnAtStation))
  ;[1 1 1] Lerp the player into the correct position while they are at the speed bag station
  (Utilities|FlowControl|Sequence
    (:then_0
      (Utilities|IsValid _pawnatstation
        (:Is%20Valid
          (if (and (Variables|SpeedBag|GetLerpPlayer) (Variables|/Game/SpeedBagContent/Blueprints/SpeedBagPawn_BP.SpeedBagPawn_BP_C|GetAtBagStation _pawnatstation))
            (Transformation|SetActorLocation (Variables|SpeedBag|GetPawnAtStation) (Math|Interpolation|VInterpTo (Transformation|GetActorLocation _pawnatstation) (Transformation|GetWorldLocation (Variables|Default|GetSphereTrigger)) DeltaSeconds 7.0) false)))))))

(fn ConstructionScript)